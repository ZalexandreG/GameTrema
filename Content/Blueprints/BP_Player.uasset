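; Player character Blueprint with camera-yaw-relative movement and jumping, which respawns after falling for too long.
; BeginPlay stores the starting transform as the respawn point.
; Tick counts consecutive falling frames, so the delay depends on frame rate, and resets the count when not falling.
; At the threshold it plays scream and explosion effects, calls player death, spawns and possesses a new BP_Player, then destroys itself.
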(event `self.ReceiveBeginPlay`
  ;[1 1 1] Begin play - Set respawn transform
  (set `self.RespawnTransform` (`self.GetTransform`)))

(event `InputAxis|MoveForward`
  (params (AxisValue :type "Float (single-precision)"))
  ;[1 1 1] ZQSD input
  (`self.AddMovementInput` (`KismetMathLibrary.GetForwardVector` (`KismetMathLibrary.MakeRotator` 0.0 0.0 (.yaw (`self.GetControlRotation`)))) AxisValue))

(event `InputAxis|MoveRight`
  (params (AxisValue :type "Float (single-precision)"))
  ;[1 1 1] ZQSD input
  (`self.AddMovementInput` (`KismetMathLibrary.GetRightVector` (`KismetMathLibrary.MakeRotator` 0.0 0.0 (.yaw (`self.GetControlRotation`)))) AxisValue))

(event `InputAction|Jump`
  (params (Key :type "Key Structure"))
  ;[1 1 1] Jump action
  (:`Pressed`
    (`self.Jump`))
  (:`Released`
    (`self.StopJumping`)))

(event `self.ReceiveTick`
  (params (DeltaSeconds :type "Float (single-precision)"))
  ;[1 1 1] Check if the player is falling - if he is, respawn the player after X seconds
  (if (`NavMovementComponent.IsFalling` (`self.CharacterMovement`))
    (`/Engine/EditorBlueprintResources/StandardMacros.IncrementFloat` (`self.FallingTimeCounter`)
      (:`  `
        (if (>= (`self.FallingTimeCounter`) 200.0)
          (`GameplayStatics.PlaySound2D` "/Game/Musics/SFX/WilhemScream_Cue.WilhemScream_Cue" 0.5 1.0 0.0 null null)
          (`GameplayStatics.SpawnEmitterAtLocation` "/Game/StarterContent/Particles/P_Explosion.P_Explosion" (`self.K2_GetActorLocation`))
          (set `self.FallingTimeCounter` 0.0)
          (`self.PlayerDeath`)
          (bind _returnvalue (`|SpawnActorFromClass` "BP_Player_C" (`self.RespawnTransform`) "Undefined" "OverrideRootScale" null null))
          (`Controller.Possess` (`GameplayStatics.GetPlayerController` 0) _returnvalue)
          (`self.K2_DestroyActor`))))
    (else
      (set `self.FallingTimeCounter` 0.0))))

(fn `UserConstructionScript`)