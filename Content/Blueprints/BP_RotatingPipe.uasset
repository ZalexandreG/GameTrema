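; BP_RotatingPipe is a spinning pipe obstacle that flings the player on contact.
; Its construction script uses IsVertical to pick the mesh orientation and scale, and a randomized spin rate on pitch or yaw for RotatingMovement.
; A capsule overlap launches BP_Player along its velocity times a random multiplier, or along a fixed diagonal if it is nearly stationary, overriding current velocity.
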(event `self.Capsule.OnComponentBeginOverlap`
  (params (OverlappedComponent :type "PrimitiveComponent Object Reference") (OtherActor :type "Actor Object Reference") (OtherComp :type "PrimitiveComponent Object Reference") (OtherBodyIndex :type Integer) (bFromSweep :type Boolean) (SweepResult :type "HitResult Structure (by ref)"))
  (bind _asbp_player (cast `/Game/Blueprints/BP_Player` OtherActor))
  (`KismetSystemLibrary.PrintString` "Player touched")
  (bind _returnvalue (`self.GetVelocity` _asbp_player))
  (if (== _returnvalue (0.0 0.0 0.0) :`ErrorTolerance` 50.0)
    (`Character.LaunchCharacter` _asbp_player (* (100.0 100.0 100.0) (`KismetMathLibrary.RandomFloatInRange` 5.0 10.0)) true true)
    (else
      (`Character.LaunchCharacter` _asbp_player (* _returnvalue (`KismetMathLibrary.RandomFloatInRange` 5.0 10.0)) true true))))

(fn `UserConstructionScript`
  (if (`self.IsVertical?`)
    (set `RotatingMovementComponent.RotationRate` (`KismetMathLibrary.MakeRotator` 0.0 (`KismetMathLibrary.RandomFloatInRange` 150.0 200.0)) (`self.RotatingMovement`))
    (`SceneComponent.K2_SetWorldRotation` :`self` (`self.StaticMesh`))
    (`SceneComponent.SetWorldScale3D` (`self.StaticMesh`) (12.5 12.5 12.5))
    (else
      (set `RotatingMovementComponent.RotationRate` (`KismetMathLibrary.MakeRotator` 0.0 0.0 (`KismetMathLibrary.RandomFloatInRange` 150.0 200.0)) (`self.RotatingMovement`))
      (`SceneComponent.K2_SetWorldRotation` (`self.StaticMesh`) (struct :`Pitch` 90.0) false false)
      (`SceneComponent.SetWorldScale3D` (`self.StaticMesh`) (6.0 6.0 6.0)))))