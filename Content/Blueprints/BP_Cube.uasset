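; BP_Cube is an actor that fades out and destroys itself when the player character touches it.
; Overlapping its Box with player 0's character starts a looping, fast timer on the Dissolve function.
; Each tick, Dissolve writes OpacityCube to the Cube's Opacity material parameter and decreases it, clearing the timer and destroying the actor at zero.
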(event `self.Box.OnComponentBeginOverlap`
  (params (OverlappedComponent :type "PrimitiveComponent Object Reference") (OtherActor :type "Actor Object Reference") (OtherComp :type "PrimitiveComponent Object Reference") (OtherBodyIndex :type Integer) (bFromSweep :type Boolean) (SweepResult :type "HitResult Structure (by ref)"))
  (if (== OtherActor (`GameplayStatics.GetPlayerCharacter` 0))
    (`KismetSystemLibrary.K2_SetTimer` null "Dissolve" 0.01 true)))

(fn `Dissolve`
  (`MeshComponent.SetScalarParameterValueOnMaterials` (`self.Cube`) "Opacity" (`self.OpacityCube`))
  (set `self.OpacityCube` (- (`self.OpacityCube`) (`self.OpacityToDecrease`)))
  (if (<= (`self.OpacityCube`) 0.0)
    (`KismetSystemLibrary.K2_ClearTimer` null "Dissolve")
    (`self.K2_DestroyActor`)))

(fn `UserConstructionScript`)